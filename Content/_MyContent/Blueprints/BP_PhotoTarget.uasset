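; BP_PhotoTarget is a photo target actor with a configurable skeletal mesh, applied in the construction script, that can slide to an end point.
; Tick checks IsMoving and calls the Move dispatcher, whose bound StartMoving event clears the flag and plays a Timeline.
; The Timeline lerps the actor from its BeginPlay location to EndPoint, with play rate derived from Duration.
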(event `self.ReceiveBeginPlay`
  (set `self.Start Point` (`self.K2_GetActorLocation`))
  (add `self.Move` (delegate `Start Moving`))
  (if (`self.isMoving?`) :!label _label
    (`self.Move`)))

(event `self.ReceiveTick`
  (params (DeltaSeconds :type "Float (single-precision)"))
  (goto _label))

(event `Start Moving`
  (set `self.isMoving?` false)
  (bind (_direction _alpha) (`Timeline|Timeline`)
    (:`Update`
      (`TimelineComponent.SetPlayRate` (`self.Timeline`) (/ 1.0 (`self.Duration`)))
      (`self.K2_SetActorLocation` (`KismetMathLibrary.VLerp` (`self.Start Point`) (`self.End Point`) _alpha)))))

(fn `UserConstructionScript`
  (`SkinnedMeshComponent.SetSkinnedAssetAndUpdate` (`self.SkeletalMeshComponent`) (`self.New Mesh`) true))